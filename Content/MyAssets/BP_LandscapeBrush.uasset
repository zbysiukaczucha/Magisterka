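; Landscape brush that generates terrain from a sound by painting a square render target.
; RunAnalysis feeds Constant-Q, loudness and onset analyzers, whose sampled results set brush roughness, radius, density and size.
; GenerateTerrain stamps a dynamic material along a square spiral or an edge-bouncing path steered by frequency balance or loudness oscillation, optionally interpolated with substeps.
; AnalyzeTerrain runs a grid raycaster walkability check and exports the heightmap as EXR.
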(fn `AnalyzeTerrain`
  (bind _gridraycaster (`self.GridRaycaster`))
  (`/Engine/EditorBlueprintResources/StandardMacros.IsValid` (`self.GridRaycaster`)
    (:`Is Valid`
      (set `/Game/MyAssets/GridRaycaster.CSV Path` (`self.CSV Path`) _gridraycaster)
      (`/Game/MyAssets/GridRaycaster.CheckWalkablePoints` _gridraycaster))
    (:`Is Not Valid`
      _))
  (`KismetRenderingLibrary.ExportRenderTarget` (`self.Texture Render Target`) (`self.Heightmaps Path`) (`KismetStringLibrary.Concat_StrStr` (`KismetSystemLibrary.GetObjectName` (`self.AnalyzedSound`)) "_" (`|GetEnumeratorNameAsString` (`self.Algorithm`)) "_" (`KismetStringLibrary.Conv_IntToString` (`self.NumberOfIterations`)) "_" (`KismetMathLibrary.SelectString` "On" "Off" (`self.EnableSubsteps`)) ".EXR")))

(fn `Draw`
  (locals (Alpha :type "Float (double-precision)"))
  (bind (_currentposition_x _currentposition_y) (`KismetMathLibrary.BreakVector2D` (`self.CurrentPosition`)))
  (bind (_previousposition_x _previousposition_y) (`KismetMathLibrary.BreakVector2D` (`self.PreviousPosition`)))
  (bind _alpha (`local.Alpha`))
  (bind _returnvalue (`KismetMathLibrary.Lerp` (`self.PreviusBrushSize`) (`self.CurrentBrushSize`) (`local.Alpha`)))
  (if (`self.EnableSubsteps`)
    (set `self.SubstepsCount` (`KismetMathLibrary.Clamp` (`KismetMathLibrary.FCeil` (/ (`KismetMathLibrary.Distance2D` (`self.PreviousPosition`) (`self.CurrentPosition`)) (* (`KismetMathLibrary.FMax` (`self.CurrentBrushSize`) 1.0) 0.01))) 1 20))
    (else
      (set `self.SubstepsCount` 1)))
  (for _index (range 1 (+ (`self.SubstepsCount`) 1))
    (set `local.Alpha` (/ (`KismetMathLibrary.Conv_IntToDouble` _index) (`KismetMathLibrary.Conv_IntToDouble` (`self.SubstepsCount`))))
    (`MaterialInstanceDynamic.SetScalarParameterValue` (`self.BrushDynamicMaterialInstance`) "Roughness" (`KismetMathLibrary.Lerp` (`self.PreviousRoughness`) (`self.CurrentRoughness`) (`local.Alpha`)))
    (`MaterialInstanceDynamic.SetScalarParameterValue` (`self.BrushDynamicMaterialInstance`) "Radius" (`KismetMathLibrary.Lerp` (`self.PreviousRadius`) (`self.CurrentRadius`) (`local.Alpha`)))
    (`MaterialInstanceDynamic.SetScalarParameterValue` (`self.BrushDynamicMaterialInstance`) "Density" (/ (`KismetMathLibrary.Lerp` (`self.PreviousDensity`) (`self.CurrentDensity`) (`local.Alpha`)) (`self.SubstepsCount`)))
    (`Canvas.K2_DrawMaterial` (`self.Canvas`) (`self.BrushDynamicMaterialInstance`) (- (`KismetMathLibrary.MakeVector2D` (`KismetMathLibrary.Lerp` _previousposition_x _currentposition_x _alpha) (`KismetMathLibrary.Lerp` _previousposition_y _currentposition_y _alpha)) (/ _returnvalue 2.0)) (`KismetMathLibrary.Conv_DoubleToVector2D` _returnvalue) (0.0 0.0) (1.0 1.0) 0.0 (0.5 0.5)))
  (set `self.PreviousRoughness` (`self.CurrentRoughness`))
  (set `self.PreviousRadius` (`self.CurrentRadius`))
  (set `self.PreviousDensity` (`self.CurrentDensity`))
  (set `self.PreviusBrushSize` (`self.CurrentBrushSize`))
  (set `self.PreviousPosition` (`self.CurrentPosition`)))

(fn `FrequencyBalance`
  (set `self.PreviousPosition` (`KismetMathLibrary.Conv_DoubleToVector2D` (/ (`self.RenderTargetSize`) 2.0)))
  (set `self.MoveDirection` (`KismetMathLibrary.GetRotated2D` (0.0 1.0) 137.5))
  (set `self.StepSize` (* (`self.RenderTargetSize`) (`self.AnalysisStep`) (/ (`self.ReferenceDuration`) (`self.Duration`)) 0.25))
  (for _index (range (`self.NumberOfIterations`))
    (bind _returnvalue (* _index (`self.AnalysisStep`)))
    (`self.SetBrushParameters` _returnvalue)
    (bind _outconstantq (`ConstantQNRT.GetNormalizedChannelConstantQAtTime` (`self.ConstantQ Analyzer`) _returnvalue 0))
    (set `self.MoveDirection` (`KismetMathLibrary.GetRotated2D` (`self.MoveDirection`) (`KismetMathLibrary.MapRangeClamped` (- (`self.GetBandAverage` _outconstantq 73 95) (`self.GetBandAverage` _outconstantq 0 34)) -1.0 1.0 -10.0 10.0)))
    (bind _output_get (set `self.CurrentPosition` (+ (`self.PreviousPosition`) (* (`self.MoveDirection`) (`self.StepSize`)))))
    (`|ExecutionSequence`
      (:`then_0`
        (if (or (< (`KismetMathLibrary.BreakVector2D` _output_get) 0.0) (> (`KismetMathLibrary.BreakVector2D` _output_get) (`self.RenderTargetSize`)))
          (`self.ChangeDirectionX`)))
      (:`then_1`
        (if (or (< (`.Y` (`KismetMathLibrary.BreakVector2D` _output_get)) 0.0) (> (`.Y` (`KismetMathLibrary.BreakVector2D` _output_get)) (`self.RenderTargetSize`)))
          (`self.ChangeDirectionY`)))
      (:`then_2`
        (`self.Draw`)))))

(fn `GenerateTerrain`
  (bind _texture_render_target (`self.Texture Render Target`))
  (bind (_returnvalue_days _returnvalue_hours _returnvalue_minutes _returnvalue_seconds _returnvalue_milliseconds) (`KismetMathLibrary.BreakTimespan` (- (`KismetMathLibrary.Now`) (`self.StartTime`))))
  (set `self.StartTime` (`KismetMathLibrary.Now`))
  (bind _output_get (set `self.Duration` (`SoundBase.Duration` (`self.AnalyzedSound`))))
  (set `self.AnalysisStep` (/ _output_get (`self.NumberOfIterations`)))
  (bind (_canvas _size _context) (`KismetRenderingLibrary.BeginDrawCanvasToRenderTarget` _texture_render_target))
  (set `self.Canvas` _canvas)
  (if (== (`KismetMathLibrary.BreakVector2D` _size) (`.Y` (`KismetMathLibrary.BreakVector2D` _size)))
    (set `self.RenderTargetSize` (`KismetMathLibrary.BreakVector2D` _size))
    (`KismetRenderingLibrary.ClearRenderTarget2D` _texture_render_target)
    (bind _returnvalue (`KismetMaterialLibrary.CreateDynamicMaterialInstance` (`self.BrushMaterial`)))
    (set `self.BrushDynamicMaterialInstance` _returnvalue)
    (`|ExecutionSequence`
      (:`then_0`
        (switch `/Game/MyAssets/SoundToTerrainAlgorithms` (`self.Algorithm`)
          (:`NewEnumerator0`
            (`self.SquareSpiral`))
          (:`NewEnumerator1`
            (`self.FrequencyBalance`))
          (:`NewEnumerator2`
            (`self.LoudnessOscillation`))))
      (:`then_1`
        (`KismetRenderingLibrary.EndDrawCanvasToRenderTarget` _context)
        (`KismetSystemLibrary.PrintString` (`KismetStringLibrary.Concat_StrStr` "Time: " (`KismetStringLibrary.Conv_IntToString` _returnvalue_milliseconds)))
        (set `self.AffectVisibilityLayer` false)
        (set `self.AffectVisibilityLayer` true)))
    (else
      (`KismetSystemLibrary.PrintString` "Invalid render target dimensions"))))

(fn `GetBandAverage`
  (params (`CQT Results` :type "Array of Float (double-precision)") (`Start Index` :type Integer) (`End Index` :type Integer))
  (returns (Average :type "Float (double-precision)"))
  (locals (Sum :type "Float (double-precision)"))
  (for _index (range `Start Index` (+ `End Index` 1))
    (set `local.Sum` (+ (`|GetArrayItem` `CQT Results` _index) (`local.Sum`))))
  (return (/ (`local.Sum`) (+ (- `End Index` `Start Index`) 1))))

(fn `GetBandSum`
  (params (`CQT Results` :type "Array of Float (double-precision)") (`Start Index` :type Integer) (`End Index` :type Integer))
  (returns (Sum :type "Float (double-precision)"))
  (locals (TempSum :type "Float (double-precision)"))
  (for _index (range `Start Index` (+ `End Index` 1))
    (set `local.TempSum` (+ (`|GetArrayItem` `CQT Results` _index) (`local.TempSum`))))
  (return (`local.TempSum`)))

(fn `LoudnessOscillation`
  (bind _rendertargetsize (`self.RenderTargetSize`))
  (set `self.PreviousPosition` (`KismetMathLibrary.Conv_DoubleToVector2D` (/ (`self.RenderTargetSize`) 2.0)))
  (set `self.MoveDirection` (`KismetMathLibrary.GetRotated2D` (0.0 1.0) 137.5))
  (set `self.StepSize` (* (`self.RenderTargetSize`) (`self.AnalysisStep`) (/ (`self.ReferenceDuration`) (`self.Duration`)) 0.25))
  (for _index (range (`self.NumberOfIterations`))
    (bind _returnvalue (* _index (`self.AnalysisStep`)))
    (`self.SetBrushParameters` _returnvalue)
    (bind _outloudness (`LoudnessNRT.GetNormalizedLoudnessAtTime` (`self.Loudness Analyzer`) _returnvalue))
    (bind _output_get (set `self.MoveDirection` (`KismetMathLibrary.GetRotated2D` (`self.MoveDirection`) (* (`KismetMathLibrary.MapRangeClamped` (`KismetMathLibrary.SelectFloat` 0.0 _outloudness (`KismetMathLibrary.Vector_IsNAN` (`KismetMathLibrary.Conv_DoubleToVector` _outloudness))) 0.0 1.0 2.0 10.0) (+ (`KismetMathLibrary.DegSin` (* _index 0.13)) (`KismetMathLibrary.DegCos` (* _index 0.37)))))))
    (bind _output_get_2 (set `self.CurrentPosition` (+ (* _output_get (`self.StepSize`)) (`self.PreviousPosition`))))
    (`|ExecutionSequence`
      (:`then_0`
        (if (or (< (`KismetMathLibrary.BreakVector2D` _output_get_2) 0.0) (> (`KismetMathLibrary.BreakVector2D` _output_get_2) _rendertargetsize))
          (`self.ChangeDirectionX`)))
      (:`then_1`
        (if (or (< (`.Y` (`KismetMathLibrary.BreakVector2D` _output_get_2)) 0.0) (> (`.Y` (`KismetMathLibrary.BreakVector2D` _output_get_2)) _rendertargetsize))
          (`self.ChangeDirectionY`)))
      (:`then_2`
        (`self.Draw`)))))

(fn `RunAnalysis`
  (bind _constantq_analyzer (`self.ConstantQ Analyzer`))
  (bind _loudness_analyzer (`self.Loudness Analyzer`))
  (bind _onset_analyzer (`self.Onset Analyzer`))
  (bind _analyzedsound (`self.AnalyzedSound`))
  (`AudioAnalyzerNRT.SetSound` _constantq_analyzer _analyzedsound)
  (`AudioAnalyzerNRT.AnalyzeAudio` _constantq_analyzer)
  (`AudioAnalyzerNRT.SetSound` _loudness_analyzer _analyzedsound)
  (`AudioAnalyzerNRT.AnalyzeAudio` _loudness_analyzer)
  (`AudioAnalyzerNRT.SetSound` _onset_analyzer _analyzedsound)
  (`AudioAnalyzerNRT.AnalyzeAudio` _onset_analyzer))

(fn `SetBrushParameters`
  (params (Timestamp :type "Float (single-precision)"))
  (locals (OnsetAvg :type "Float (double-precision)"))
  (bind _onsetavg (`local.OnsetAvg`))
  (bind _outloudness (`LoudnessNRT.GetLoudnessAtTime` (`self.Loudness Analyzer`) Timestamp))
  (bind _outconstantq (`ConstantQNRT.GetNormalizedChannelConstantQAtTime` (`self.ConstantQ Analyzer`) Timestamp 0))
  (bind _returnvalue (/ (`self.AnalysisStep`) 2.0))
  (bind _sum (`self.GetBandSum` _outconstantq 73 95))
  (bind (_outonsettimestamps _outonsetstrengths) (`OnsetNRT.GetChannelOnsetsBetweenTimes` (`self.Onset Analyzer`) (- Timestamp _returnvalue) (+ _returnvalue Timestamp) 0))
  (bind _returnvalue_2 (`KismetArrayLibrary.Array_Length` _outonsetstrengths))
  (bind _returnvalue_3 (`KismetMathLibrary.MapRangeClamped` (`KismetMathLibrary.SelectFloat` -80.0 _outloudness (`KismetMathLibrary.Vector_IsNAN` (`KismetMathLibrary.Conv_DoubleToVector` _outloudness))) -80.0 -10.0 0.0 1.0))
  (for _array_element _outonsetstrengths
    (set `local.OnsetAvg` (+ _array_element (`local.OnsetAvg`))))
  (if (!= _returnvalue_2 0)
    (set `local.OnsetAvg` (/ (`local.OnsetAvg`) _returnvalue_2))
    (else
      (set `local.OnsetAvg` 0.0)))
  (set `self.CurrentRoughness` (`KismetMathLibrary.MapRangeClamped` (/ _sum (+ _sum (`self.GetBandSum` _outconstantq 0 34) 0.0001)) 0.0 0.45 0.0 1.0))
  (set `self.CurrentRadius` _returnvalue_3)
  (set `self.CurrentDensity` (* (/ (`self.ReferenceDuration`) (`self.Duration`)) _returnvalue_3 _returnvalue_3 (`KismetMathLibrary.MapRangeClamped` _onsetavg 0.0 50.0 0.05 1.0)))
  (set `self.CurrentBrushSize` (* (* _returnvalue_3 (`KismetMathLibrary.MapRangeClamped` _onsetavg 0.0 50.0 1.0 2.0)) (/ (`self.RenderTargetSize`) 2.0))))

(fn `SquareSpiral`
  (locals (DirectionIndex :type Integer) (StepsTaken :type Integer) (CurrentLineLength :type Integer :default 1) (TurnCount :type Integer))
  (bind _numberofiterations (`self.NumberOfIterations`))
  (bind (_previousposition_x _previousposition_y) (`KismetMathLibrary.BreakVector2D` (`self.PreviousPosition`)))
  (bind (_previousposition_x_2 _previousposition_y_2) (`KismetMathLibrary.BreakVector2D` (`self.PreviousPosition`)))
  (bind (_previousposition_x_3 _previousposition_y_3) (`KismetMathLibrary.BreakVector2D` (`self.PreviousPosition`)))
  (bind (_previousposition_x_4 _previousposition_y_4) (`KismetMathLibrary.BreakVector2D` (`self.PreviousPosition`)))
  (set `self.PreviousPosition` (`KismetMathLibrary.Conv_DoubleToVector2D` (/ (`self.RenderTargetSize`) 2.0)))
  (set `self.StepSize` (/ (`self.RenderTargetSize`) (`KismetMathLibrary.Sqrt` (`KismetMathLibrary.Conv_IntToDouble` _numberofiterations))))
  (for _index (range _numberofiterations)
    (`self.SetBrushParameters` (* _index (`self.AnalysisStep`)))
    (switch `int` (`local.DirectionIndex`)
      (:`0`
        (set `self.CurrentPosition` (`KismetMathLibrary.MakeVector2D` (+ _previousposition_x_4 (`self.StepSize`)) _previousposition_y_4)))
      (:`1`
        (set `self.CurrentPosition` (`KismetMathLibrary.MakeVector2D` _previousposition_x (+ _previousposition_y (`self.StepSize`)))))
      (:`2`
        (set `self.CurrentPosition` (`KismetMathLibrary.MakeVector2D` (- _previousposition_x_3 (`self.StepSize`)) _previousposition_y_3)))
      (:`3`
        (set `self.CurrentPosition` (`KismetMathLibrary.MakeVector2D` _previousposition_x_2 (- _previousposition_y_2 (`self.StepSize`))))))
    (`self.Draw`)
    (bind _result (`/Engine/EditorBlueprintResources/StandardMacros.IncrementInt` (`local.StepsTaken`))
      (:`  `
        (if (>= _result (`local.CurrentLineLength`))
          (set `local.StepsTaken` 0)
          (set `local.DirectionIndex` (mod (+ (`local.DirectionIndex`) 1) 4))
          (bind _result_2 (`/Engine/EditorBlueprintResources/StandardMacros.IncrementInt` (`local.TurnCount`))
            (:`  `
              (if (== _result_2 2)
                (`/Engine/EditorBlueprintResources/StandardMacros.IncrementInt` (`local.CurrentLineLength`)
                  (:`  `
                    (set `local.TurnCount` 0)))))))))))

(fn `UserConstructionScript`
  (`parent.UserConstructionScript`)
  (bind _returnvalue (`KismetMaterialLibrary.CreateDynamicMaterialInstance` "/Game/MyAssets/GenNoise_Audio.GenNoise_Audio"))
  (`MaterialInstanceDynamic.SetTextureParameterValue` _returnvalue "AudioInput" (`self.Texture Render Target`)))